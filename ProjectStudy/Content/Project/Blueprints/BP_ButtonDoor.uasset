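; BP_ButtonDoor is a door actor that swings when something overlaps its Box trigger.
; The overlap calls ShiftSwitch if SwichDoor is false, playing the Open timeline to drive the door's yaw.
; On completion, SetEventFlnshed calls its parent, zeroes the door's rotation and disables Box collision.
; SwichDoor is only ever set false here, so this file never blocks retriggering during the swing.
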(event `self.ReceiveBeginPlay`
  (`parent.ReceiveBeginPlay`))

(event `Shift Switch`
  (set `self.SwichDoor` false)
  (bind (_direction _open_z) (`Timeline|Open`)
    (:`Update`
      (`SceneComponent.K2_SetRelativeRotation` (`self.Door`) (`KismetMathLibrary.MakeRotator` 0.0 0.0 _open_z) false false))
    (:`Finished`
      (`self.SetEventFlnshed`))))

(event `self.Box.OnComponentBeginOverlap`
  (params (OverlappedComponent :type "PrimitiveComponent Object Reference") (OtherActor :type "Actor Object Reference") (OtherComp :type "PrimitiveComponent Object Reference") (OtherBodyIndex :type Integer) (bFromSweep :type Boolean) (SweepResult :type "HitResult Structure (by ref)"))
  (if (not (`self.SwichDoor`))
    (`self.Shift Switch`)))

(fn `SetEventFlnshed`
  (`parent.SetEventFlnshed`)
  (set `self.SwichDoor` false)
  (`SceneComponent.K2_SetRelativeRotation` :`self` (`self.Door`))
  (`PrimitiveComponent.SetCollisionEnabled` (`self.Box`) "NoCollision"))

(fn `UserConstructionScript`)