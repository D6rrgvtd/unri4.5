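; BP_Door is a door that swings open on a timeline-driven yaw, with behavior selected by DoorType.
; When BP_Player overlaps its Box, a Key door opens if KeyName is None or BP_MyGameinstance reports the key as Got, saving it as Used.
; A Lever door instead calls ShiftLever on TargetLever.
; A separate OpenDoor event opens it through a second timeline and calls SetEventFlnshed when finished.
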(event `self.ReceiveBeginPlay`
  (`parent.ReceiveBeginPlay`))

(event `self.Box.OnComponentBeginOverlap`
  (params (OverlappedComponent :type "PrimitiveComponent Object Reference") (OtherActor :type "Actor Object Reference") (OtherComp :type "PrimitiveComponent Object Reference") (OtherBodyIndex :type Integer) (bFromSweep :type Boolean) (SweepResult :type "HitResult Structure (by ref)"))
  (cast `/Game/Project/Blueprints/BP_Player` OtherActor)
  (switch `/Game/Project/Data/E_DoorType` (`self.DoorType`)
    (:`NewEnumerator0`
      (bind _asbp_my_gameinstance (cast `/Game/Project/Blueprints/BP_MyGameinstance` (`GameplayStatics.GetGameInstance`)))
      (if (== (`self.KeyName`) "None")
        (bind (_direction _openz) (`Timeline|Open` :!label _label)
          (:`Update`
            (`SceneComponent.K2_SetRelativeRotation` (`self.Door`) (`KismetMathLibrary.MakeRotator` 0.0 0.0 _openz) false false)))
        (else
          (switch `/Game/Project/Data/EN_KeyStatus` (`/Game/Project/Blueprints/BP_MyGameinstance.GetKeyStatus` _asbp_my_gameinstance (`self.KeyName`))
            (:`NewEnumerator1`
              (`/Game/Project/Blueprints/BP_MyGameinstance.SaveKeyStatus` _asbp_my_gameinstance (`self.KeyName`) "NewEnumerator2")
              (goto _label))))))
    (:`NewEnumerator2`
      (`/Game/Project/Blueprints/BP_Lever.ShiftLever` (`self.Target Lever`)))))

(event `Open Door`
  (bind (_direction _openz) (`Timeline|タイムライン_0`)
    (:`Update`
      (`SceneComponent.K2_SetRelativeRotation` (`self.Door`) (`KismetMathLibrary.MakeRotator` 0.0 0.0 _openz) false false))
    (:`Finished`
      (`self.SetEventFlnshed`))))

(fn `UserConstructionScript`)