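; BP_SwitchButton is a switch button that, when triggered by an overlapping component, can open a target door and start a target box moving.
; A tag-checked Box overlap plays the SwitchOn timeline to animate the button mesh, then calls OpenDoor and activates the box's InterpToMovement on valid targets.
; Only the door branch calls SetEventFlnshed, which runs the parent logic, sets the button's relative location to zero and disables trigger collision.
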(event `self.ReceiveBeginPlay`
  (`parent.ReceiveBeginPlay`))

(event `self.Box.OnComponentBeginOverlap`
  (params (OverlappedComponent :type "PrimitiveComponent Object Reference") (OtherActor :type "Actor Object Reference") (OtherComp :type "PrimitiveComponent Object Reference") (OtherBodyIndex :type Integer) (bFromSweep :type Boolean) (SweepResult :type "HitResult Structure (by ref)"))
  (if (`ActorComponent.ComponentHasTag` OtherComp "None")
    (bind (_direction _buttonz) (`Timeline|SwitchOn`)
      (:`Update`
        (`SceneComponent.K2_SetRelativeLocation` (`self.STM_Button`) (`KismetMathLibrary.Conv_DoubleToVector` _buttonz) false false))
      (:`Finished`
        (`|ExecutionSequence`
          (:`then_0`
            (bind _targetdoor (`self.TargetDoor`)
              (:`then`
                (`/Game/Project/Blueprints/BP_Door.Open Door` _targetdoor)
                (`self.SetEventFlnshed`))
              (:`else`)))
          (:`then_1`
            (bind _targetbox (`self.TargetBox`)
              (:`then`
                (`ActorComponent.SetActive` (`/Game/Project/Blueprints/BP_MovingBox.InterpToMovement` _targetbox) true false))
              (:`else`))))))))

(fn `SetEventFlnshed`
  (`parent.SetEventFlnshed`)
  (`SceneComponent.K2_SetRelativeLocation` (`self.STM_Button`) (0.0 0.0 0.0) false false)
  (`PrimitiveComponent.SetCollisionEnabled` (`self.Box`) "NoCollision"))

(fn `UserConstructionScript`)