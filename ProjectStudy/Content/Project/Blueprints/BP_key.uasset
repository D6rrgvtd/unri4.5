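; BP_key is a key pickup actor that registers itself as obtained when a tagged component overlaps its sphere.
; On overlap, it checks the component for the tag "None", notifies the player through ACOverlapPlayer and saves the key's status by KeyName in the game instance.
; It then calls SetEventFlnshed, an override that runs the parent's event-completion logic before destroying the actor.
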(event `self.ReceiveBeginPlay`
  (`parent.ReceiveBeginPlay`))

(event `self.Sphere.OnComponentBeginOverlap`
  (params (OverlappedComponent :type "PrimitiveComponent Object Reference") (OtherActor :type "Actor Object Reference") (OtherComp :type "PrimitiveComponent Object Reference") (OtherBodyIndex :type Integer) (bFromSweep :type Boolean) (SweepResult :type "HitResult Structure (by ref)"))
  (if (`ActorComponent.ComponentHasTag` OtherComp "None")
    (`/Game/Project/Blueprints/AC_OverlapPlayer.NotifyToPlayer` (`self.AC Overlap Player`) null (`self.KeyName`))
    (`/Game/Project/Blueprints/BP_MyGameinstance.SaveKeyStatus` (`self.MyGameInstance`) (`self.KeyName`) "NewEnumerator1")
    (`self.SetEventFlnshed`)))

(fn `SetEventFlnshed`
  (`parent.SetEventFlnshed`)
  (`self.K2_DestroyActor`))

(fn `UserConstructionScript`)