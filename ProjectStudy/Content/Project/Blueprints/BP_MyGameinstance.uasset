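; Game instance that keeps event and key progress states across level loads.
; Save and get functions write to and read from two name-keyed maps, returning the first enum entry when a name is missing.
; GoalEvent clears both maps, waits briefly, then reloads the current level to restart with fresh state.
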(event `GoalEvent`
  (`BlueprintMapLibrary.Map_Clear` (`self.Event Status`))
  (`BlueprintMapLibrary.Map_Clear` (`self.KeyStatus`))
  (`KismetSystemLibrary.Delay` 2.0)
  (bind _returnvalue (`GameplayStatics.GetCurrentLevelName` true))
  (`GameplayStatics.OpenLevel` (`KismetStringLibrary.Conv_StringToName` _returnvalue)))

(fn `GetEventStatus`
  (params (`Event Name` :type Name))
  (returns (Status :type "/Game/Project/Data/EN_EventStatus Enum"))
  (bind (_value _returnvalue) (`BlueprintMapLibrary.Map_Find` (`self.Event Status`) `Event Name`))
  (if _returnvalue
    (return _value)
    (else
      (return "NewEnumerator0"))))

(fn `GetKeyStatus`
  (params (`Key Name` :type Name))
  (returns (Status :type "/Game/Project/Data/EN_KeyStatus Enum"))
  (bind (_value _returnvalue) (`BlueprintMapLibrary.Map_Find` (`self.KeyStatus`) `Key Name`))
  (if _returnvalue
    (return _value)
    (else
      (return "NewEnumerator0"))))

(fn `SaveEventStatus`
  (params (`Event Name` :type Name) (Status :type "/Game/Project/Data/EN_EventStatus Enum" :default "NewEnumerator0"))
  (`BlueprintMapLibrary.Map_Add` (`self.Event Status`) `Event Name` Status))

(fn `SaveKeyStatus`
  (params (`Key Name` :type Name) (Status :type "/Game/Project/Data/EN_KeyStatus Enum" :default "NewEnumerator0"))
  (`BlueprintMapLibrary.Map_Add` (`self.KeyStatus`) `Key Name` (cast `/Game/Project/Data/EN_KeyStatus` Status)))