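; BP_EventBase is an event actor, apparently a base class, that tracks its completion status through BP_MyGameinstance.
; The construction script derives the EventName key from the actor's display name.
; On BeginPlay it looks up that key, re-applying Finished through SetEventFlnshed, or otherwise saving the event as Unfinished.
; SetEventFlnshed marks the event Finished and saves it to the game instance.
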(event `self.ReceiveBeginPlay`
  (bind _asbp_my_gameinstance (cast `/Game/Project/Blueprints/BP_MyGameinstance` (`GameplayStatics.GetGameInstance`)))
  (bind _output_get (set `self.My Game instance` _asbp_my_gameinstance))
  (bind _output_get_2 (set `self.EventStatus` (`/Game/Project/Blueprints/BP_MyGameinstance.GetEventStatus` _output_get (`self.Event Name`))))
  (switch `/Game/Project/Data/EN_EventStatus` _output_get_2
    (:`NewEnumerator0`
      (bind _output_get_3 (set `self.EventStatus` "NewEnumerator1"))
      (`/Game/Project/Blueprints/BP_MyGameinstance.SaveEventStatus` (`self.My Game instance`) (`self.Event Name`) _output_get_3))
    (:`NewEnumerator2`
      (`self.SetEventFlnshed`))))

(fn `SetEventFlnshed`
  (bind _output_get (set `self.EventStatus` "NewEnumerator2"))
  (`/Game/Project/Blueprints/BP_MyGameinstance.SaveEventStatus` (`self.My Game instance`) (`self.Event Name`) _output_get))

(fn `UserConstructionScript`
  (set `self.Event Name` (`KismetStringLibrary.Conv_StringToName` (`KismetSystemLibrary.GetDisplayName` self))))